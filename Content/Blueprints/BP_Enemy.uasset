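; Paper2D Bringer of Death enemy that patrols forward, turning around at walls and ledges via detector overlaps.
; Player overlap with its sphere makes the enemy damage itself and play a hurt flipbook.
; AnyDamage scales damage by 100, lowers health and updates the health-bar widget.
; After a delay, health thresholds restore walking or stop movement, play death and destroy the actor.
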(event OnComponentBeginOverlap(Sphere)
  (params (OverlappedComponent :type Primitive%20Component%20Object%20Reference) (OtherActor :type Actor%20Object%20Reference) (OtherComp :type Primitive%20Component%20Object%20Reference) (OtherBodyIndex :type Integer) (bFromSweep :type Boolean) (SweepResult :type Hit%20Result%20Structure%20%28by%20ref%29))
  (Utilities|Casting|CastToPP_Player OtherActor)
  (Game|Damage|ApplyDamage self 1.0 0 0)
  (Sprite|SetFlipbook (Variables|Default|GetSprite) "/Game/Assets/Bringer-Of-Death/Individual_Sprite/Hurt/Bringer-of-Death_Hurt.Bringer-of-Death_Hurt")
  (Utilities|FlowControl|Delay 0.5)
  (if (<= (Variables|Default|GetCurrentHealth) 500)
    (Sprite|SetFlipbook (Variables|Default|GetSprite) "/Game/Assets/Bringer-Of-Death/Individual_Sprite/Walk/Bringer-of-Death_Walk.Bringer-of-Death_Walk")
    (if (<= (Variables|Default|GetCurrentHealth) 1)
      (Pawn|Components|CharacterMovement|DisableMovement (Variables|Character|GetCharacterMovement))
      (Sprite|SetFlipbook (Variables|Default|GetSprite) "/Game/Assets/Bringer-Of-Death/Individual_Sprite/Death/Bringer-of-Death_Death.Bringer-of-Death_Death")
      (Utilities|FlowControl|Delay 1.6)
      (Actor|DestroyActor))))

(event OnComponentBeginOverlap(WallDetector)
  (params (OverlappedComponent :type Primitive%20Component%20Object%20Reference) (OtherActor :type Actor%20Object%20Reference) (OtherComp :type Primitive%20Component%20Object%20Reference) (OtherBodyIndex :type Integer) (bFromSweep :type Boolean) (SweepResult :type Hit%20Result%20Structure%20%28by%20ref%29))
  (CallFunction|TurnChar))

(event OnComponentEndOverlap(FallDetector)
  (params (OverlappedComponent :type Primitive%20Component%20Object%20Reference) (OtherActor :type Actor%20Object%20Reference) (OtherComp :type Primitive%20Component%20Object%20Reference) (OtherBodyIndex :type Integer))
  (CallFunction|TurnChar))

(event EventTick
  (params (DeltaSeconds :type Float%20%28single-precision%29))
  (Pawn|Input|AddMovementInput (Transformation|GetActorForwardVector) 1.0 false))

(event EventBeginPlay
  (bind _asbwp_enemy_health (Utilities|Casting|CastToBWP_EnemyHealth (UserInterface|GetUserWidgetObject (Variables|Default|GetWidget))))
  (bind _output_get (Variables|Default|SetAs%20BWP%20Enemy%20Health _asbwp_enemy_health))
  (Variables|/Game/UI/BWP_EnemyHealth.BWP_EnemyHealth_C|SetCurrentHealth _output_get (Variables|Default|GetCurrentHealth))
  (Variables|/Game/UI/BWP_EnemyHealth.BWP_EnemyHealth_C|SetMaxHealth _output_get (Variables|Default|GetMaxHealth)))

(event Game|Damage|EventAnyDamage
  (params (Damage :type Float%20%28single-precision%29) (DamageType :type Damage%20Type%20Object%20Reference) (InstigatedBy :type Controller%20Object%20Reference) (DamageCauser :type Actor%20Object%20Reference))
  (bind _output_get (Variables|Default|SetCurrentHealth (- (Variables|Default|GetCurrentHealth) (* Damage 1e+02))))
  (Default|UptHealth (Variables|Default|GetAs%20BWP%20Enemy%20Health) (Math|Integer|Clamp(Integer) _output_get 0 (Variables|Default|GetMaxHealth))))

(fn ConstructionScript)

(fn TurnChar
  (Transformation|SetActorRotation (Math|Rotator|CombineRotators (Transformation|GetActorRotation) "0.000000,180.000000,0.000000")))