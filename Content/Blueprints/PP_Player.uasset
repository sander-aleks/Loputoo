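; Paper2D player character with flipbook-animated movement, jump and melee attack, plus health HUD, pause menu and death screen.
; Attacks damage HitBox overlaps on flipbook frame 4, and landing speed sets tiered fall damage through AnyDamage.
; Zero health disables control, while respawn either resets at PlayerStart or, on destruction, goes through the game mode.
; G and J save and restore position, and a looping MultiGate on Tick alternates attack checks with a frame-based timer.
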(event OnFinishedPlaying(Sprite)
  (Sprite|SetFlipbook (Variables|Default|GetSprite) "/Game/Assets/FB_idle.FB_idle")
  (CallFunction|RestartAnim (Variables|Default|GetSprite))
  (Variables|Default|SetIsAttacing false)
  (CallFunction|ResetAttack)
  (Development|SetHiddeninGame (Variables|Default|GetHitBox) true false))

(event Custom|Death2
  (bind _returnvalue (Game|GetPlayerController 0))
  (Variables|Default|SetbDeath true)
  (Sprite|SetFlipbook (Variables|Default|GetSprite) "/Game/Assets/FB_death.FB_death")
  (Widget|RemovefromParent (Variables|Default|GetWB_Main))
  (bind _returnvalue_2 (UserInterface|CreateWidget "/Game/UI/WB_Death.WB_Death_C"))
  (UserInterface|Viewport|AddtoViewport _returnvalue_2 0)
  (UserInterface|Animation|PlayAnimation _returnvalue_2 (Variables|/Game/UI/WB_Death.WB_Death_C|GetImageAnimation _returnvalue_2) 0.0 1 "Forward" 1.0 false)
  (Pawn|Components|CharacterMovement|DisableMovement (Variables|Character|GetCharacterMovement))
  (Input|DisableInput 0)
  (Variables|/Script/Engine.PlayerController|SetbShowMouseCursor _returnvalue true)
  (Input|SetInputModeGameandUI _returnvalue 0 "DoNotLock" true false))

(event Custom|Death
  (Actor|DestroyActor))

(event Custom|Respawn
  (Variables|Default|SetbDeath false)
  (bind _returnvalue (Actor|GetActorOfClass "/Script/Engine.PlayerStart"))
  (Transformation|SetActorLocation (Transformation|GetActorLocation _returnvalue) false false)
  (Pawn|Components|CharacterMovement|SetMovementMode (Variables|Character|GetCharacterMovement) "MOVE_Walking" 0)
  (Sprite|SetFlipbook (Variables|Default|GetSprite) "/Game/Assets/FB_idle.FB_idle")
  (CallFunction|InitializeHealth))

(event Custom|InitializeHealth
  (bind _output_get (Variables|Default|SetCurrentHealth (Variables|Default|GetMaxHealth)))
  (Default|UpdateHealthUI (Variables|Default|GetWB_Main) _output_get (Variables|Default|GetMaxHealth)))

(event Custom|ResetAttack
  (Utilities|FlowControl|DoOnce false) ; enters at Reset
)

(event Custom|FallDamage
  (if (AI|Components|NavMovement|IsFalling (Variables|Character|GetCharacterMovement))
    (if (> (* (.z (Transformation|GetVelocity)) -1.0) 1e+03)
      (if (> (* (.z (Transformation|GetVelocity)) -1.0) 1.5e+03)
        (if (> (* (.z (Transformation|GetVelocity)) -1.0) 2e+03)
          (bind _output_get (Variables|Default|SetFallDmg 5e+01))
          (Game|Damage|ApplyDamage self _output_get (Game|GetPlayerController 0) self)
          (Development|PrintString "BigDMG")
          (else
            (bind _output_get_2 (Variables|Default|SetFallDmg 25.0))
            (Game|Damage|ApplyDamage self _output_get_2 (Game|GetPlayerController 0) self)
            (Development|PrintString "MediumDMG")))
        (else
          (bind _output_get_3 (Variables|Default|SetFallDmg 1e+01))
          (Game|Damage|ApplyDamage self _output_get_3 (Game|GetPlayerController 0) self)
          (Development|PrintString "SmallDMG"))))))

(event Input|EnhancedActionEvents|EnhancedInputActionIA_movement
  (params (ActionValue :type Float%20%28double-precision%29) (ElapsedSeconds :type Float%20%28double-precision%29) (TriggeredSeconds :type Float%20%28double-precision%29) (InputAction :type Input%20Action%20Object%20Reference :default "/Game/Blueprints/IA_movement.IA_movement"))
  (:Triggered
    (if (not (Variables|Default|GetbtsJumping))
      (Pawn|Input|AddMovementInput (Transformation|GetActorForwardVector) ActionValue false)
      (Sprite|SetFlipbook (Variables|Default|GetSprite) "/Game/Assets/FB_run.FB_run")
      (if (> ActionValue 0.0)
        (Transformation|SetWorldRotation (Variables|Default|GetSprite) "0.000000,-180.000000,0.000000" false false)
        (Utilities|FlowControl|Delay 0.3)
        (Audio|PlaySound2D "/Game/Sound/GRASS_-_Walk_1.GRASS_-_Walk_1" 0.2 1.0 0.0 0 0)
        (else
          (Transformation|SetWorldRotation (Variables|Default|GetSprite) "0, 0, 0" false false)
          (Utilities|FlowControl|Delay 0.3)
          (Audio|PlaySound2D "/Game/Sound/GRASS_-_Walk_1.GRASS_-_Walk_1" 0.2 1.0 0.0 0 0)))))
  (:Completed
    (if (not (Variables|Default|GetbtsJumping))
      (Sprite|SetFlipbook (Variables|Default|GetSprite) "/Game/Assets/FB_idle.FB_idle"))))

(event Input|EnhancedActionEvents|EnhancedInputActionIA_Jump
  (params (ActionValue :type Boolean) (ElapsedSeconds :type Float%20%28double-precision%29) (TriggeredSeconds :type Float%20%28double-precision%29) (InputAction :type Input%20Action%20Object%20Reference :default "/Game/Blueprints/IA_Jump.IA_Jump"))
  (bind _sprite (Variables|Default|GetSprite))
  (if (not (Variables|Default|GetbtsJumping))
    (Variables|Default|SetbtsJumping false)
    (Character|Jump)
    (Components|Timeline|SetLooping _sprite true)
    (Sprite|SetFlipbook _sprite "/Game/Assets/FB_jump.FB_jump")
    (Utilities|FlowControl|Delay 1.0)
    (if (== (.Z (Math|Vector|BreakVector (Transformation|GetVelocity))) 0.0) :!label _label
      (if (Variables|Default|GetbDeath) :!label _label_2
        (Utilities|FlowControl|Delay 0.1)
        (goto _label_2)
        (else
          (Components|Timeline|SetLooping _sprite true)
          (Audio|Components|Audio|Play _sprite)
          (Sprite|SetFlipbook _sprite "/Game/Assets/FB_idle.FB_idle")
          (Variables|Default|SetbtsJumping false)))
      (else
        (Utilities|FlowControl|Delay 0.1)
        (goto _label)))))

(event Input|EnhancedActionEvents|EnhancedInputActionIA_Pause
  (params (ActionValue :type Boolean) (ElapsedSeconds :type Float%20%28double-precision%29) (TriggeredSeconds :type Float%20%28double-precision%29) (InputAction :type Input%20Action%20Object%20Reference :default "/Game/Blueprints/IA_Pause.IA_Pause"))
  (bind _returnvalue (Game|GetPlayerController 0))
  (:Started
    (bind _returnvalue_2 (UserInterface|CreateWidget "/Game/UI/WB_PauseMenu.WB_PauseMenu_C"))
    (UserInterface|Viewport|AddtoViewport _returnvalue_2 0)
    (Variables|/Script/Engine.PlayerController|SetbShowMouseCursor _returnvalue true)
    (Input|SetInputModeUIOnly _returnvalue 0 "DoNotLock" false)
    (Game|SetGamePaused true)))

(event EventBeginPlay
  (Input|SetInputModeGameOnly (Game|GetPlayerController 0) false)
  (Utilities|FlowControl|MultiGate false false -1
    (:Out%200
      (Audio|PlaySound2D "/Game/Sound/forest-ambience-with-cuckoo-birds-chirping-123046__online-audio-converter_com_.forest-ambience-with-cuckoo-birds-chirping-123046__online-audio-converter_com_" 2.0 1.0 0.0 0 0)
      (bind _asbp_playercontroller (Utilities|Casting|CastToBP_playercontroller (Pawn|GetController)))
      (Input|AddMappingContext (PlayerController|LocalPlayerSubsystems|GetEnhancedInputLocalPlayerSubsystem _asbp_playercontroller) "/Game/Blueprints/IMC_default.IMC_default" 0 "(bIgnoreAllPressedKeysUntilRelease=True,bForceImmediately=False,bNotifyUserSettings=False)")
      (bind _returnvalue (UserInterface|CreateWidget "/Game/UI/WB_Main.WB_Main_C" (Game|GetPlayerController 0)))
      (bind _output_get (Variables|Default|SetWB_Main _returnvalue))
      (UserInterface|Viewport|AddtoViewport _output_get 0)
      (CallFunction|InitializeHealth))
    (:Out%201
      (bind _returnvalue_2 (SaveGame|DoesSaveGameExist "save1"))
      (if _returnvalue_2
        (bind _returnvalue_3 (SaveGame|LoadGamefromSlot "save1"))
        (bind _asbp_save (Utilities|Casting|CastToBP_Save _returnvalue_3))
        (Variables|Default|SetBP%20Save _asbp_save)
        (Transformation|SetActorTransform (Variables|/Game/Blueprints/BP_Save.BP_Save_C|GetPlayerPos _asbp_save))
        (else
          (bind _returnvalue_4 (SaveGame|CreateSaveGameObject "/Game/Blueprints/BP_Save.BP_Save_C"))
          (Variables|/Game/Blueprints/BP_Save.BP_Save_C|SetPlayerPos _returnvalue_4 (Transformation|GetActorTransform))
          (SaveGame|SaveGametoSlot _returnvalue_4 "save1")
          (Variables|Default|SetBP%20Save _returnvalue_4))))))

(event EventDestroyed
  (bind _outactors (Actor|GetAllActorsOfClass "/Game/Blueprints/BP_SpawnPoint.BP_SpawnPoint_C"))
  (bind _asbp_gamemode (Utilities|Casting|CastToBP_gamemode (Game|GetGameMode)))
  (Default|Respawn _asbp_gamemode (Transformation|GetActorTransform (Utilities|Array|Get(acopy) _outactors))))

(event Game|Damage|EventAnyDamage
  (params (Damage :type Float%20%28single-precision%29) (DamageType :type Damage%20Type%20Object%20Reference) (InstigatedBy :type Controller%20Object%20Reference) (DamageCauser :type Actor%20Object%20Reference))
  (if (not (Variables|Default|GetbDeath))
    (bind _output_get (Variables|Default|SetCurrentHealth (Math|Float|Clamp(Float) (- (Variables|Default|GetCurrentHealth) Damage) 0.0 (Variables|Default|GetMaxHealth))))
    (Default|UpdateHealthUI (Variables|Default|GetWB_Main) _output_get (Variables|Default|GetMaxHealth))
    (Effects|SpawnEmitteratLocation 0 (Transformation|GetActorLocation))
    (if (== (Variables|Default|GetCurrentHealth) 0.0)
      (CallFunction|Death2))))

(event EventOnLanded
  (params (Hit :type Hit%20Result%20Structure%20%28by%20ref%29))
  (CallFunction|FallDamage))

(event EventTick
  (params (DeltaSeconds :type Float%20%28single-precision%29))
  (Utilities|FlowControl|MultiGate false true -1
    (:Out%200
      (if (Variables|Default|GetIsAttacing)
        (if (== (Class|PaperFlipbookComponent|GetPlaybackPositioninFrames (Variables|Default|GetSprite)) 4)
          (Utilities|FlowControl|DoOnce false
            (:Completed
              (CallFunction|HitCheck))))))
    (:Out%201
      (Variables|Default|SetMilliseconds (+ (Variables|Default|GetMilliseconds) 21))
      (if (> (Variables|Default|GetMilliseconds) 999)
        (Variables|Default|SetMilliseconds 0)
        (Variables|Default|SetSeconds (+ (Variables|Default|GetSeconds) 1))
        (if (> (Variables|Default|GetSeconds) 59)
          (Variables|Default|SetMinutes (+ (Variables|Default|GetMinutes) 1))
          (Variables|Default|SetSeconds 0))))))

(event Input|KeyboardEvents|G
  (params (Key :type Key%20Structure :default "None"))
  (bind _bp_save (Variables|Default|GetBP%20Save))
  (:Pressed
    (bind _returnvalue (SaveGame|DoesSaveGameExist "save1"))
    (if _returnvalue
      (Variables|/Game/Blueprints/BP_Save.BP_Save_C|SetPlayerPos _bp_save (Transformation|GetActorTransform))
      (SaveGame|SaveGametoSlot _bp_save "save1")
      (Development|PrintString "GAME SAVED"))))

(event Input|KeyboardEvents|SpaceBar
  (params (Key :type Key%20Structure :default "None"))
  (:Pressed
    (Sprite|SetFlipbook (Variables|Default|GetSprite) "/Game/Assets/FB_attack.FB_attack")
    (Components|Timeline|SetLooping (Variables|Default|GetSprite) false)
    (Variables|Default|SetIsAttacing true)))

(event Input|KeyboardEvents|J
  (params (Key :type Key%20Structure :default "None"))
  (:Pressed
    (bind _returnvalue (SaveGame|DoesSaveGameExist "save1"))
    (if _returnvalue
      (Transformation|SetActorTransform (Variables|/Game/Blueprints/BP_Save.BP_Save_C|GetPlayerPos (Variables|Default|GetBP%20Save)))
      (Development|PrintString "GAME LOADED"))))

(event Custom|Event%20Tick
  (params (DeltaSeconds :type Float%20%28single-precision%29)))

(fn ConstructionScript)

(fn RestartAnim
  (params (self2 :type Paper%20Flipbook%20Component%20Object%20Reference))
  (Components|Timeline|SetLooping self2 true)
  (if (not (Audio|Components|Audio|IsPlaying (Variables|Default|GetSprite)))
    (Audio|Components|Audio|Play (Variables|Default|GetSprite))))

(fn HitCheck
  (for _array_element (Collision|GetOverlappingActors (Variables|Default|GetHitBox) 0 :!class /Script/Engine.PrimitiveComponent)
    (if (!= _array_element self)
      (Game|Damage|ApplyDamage _array_element (Variables|Default|GetDamage%20Amount) 0 0))))