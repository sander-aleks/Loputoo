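; BP_Enemy1 is an enemy Blueprint with basic helpers for turning and dealing hit damage.
; HitCheck applies DamageAmount to every other actor overlapping its HitBox, and TurnChar flips the actor's rotation by a half turn; neither is called within this Blueprint.
; Incoming damage is only printed for debugging, with no health tracking, and the Death event destroys the actor.
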(event Custom|Death
  (Actor|DestroyActor))

(event Game|Damage|EventAnyDamage
  (params (Damage :type Float%20%28single-precision%29) (DamageType :type Damage%20Type%20Object%20Reference) (InstigatedBy :type Controller%20Object%20Reference) (DamageCauser :type Actor%20Object%20Reference))
  (Development|PrintString (Utilities|String|ToString(Float) Damage)))

(fn ConstructionScript)

(fn TurnChar
  (Transformation|SetActorRotation (Math|Rotator|CombineRotators (Transformation|GetActorRotation) "0.000000,180.000000,0.000000")))

(fn HitCheck
  (for _array_element (Collision|GetOverlappingActors (Variables|Default|GetHitBox) 0 :!class /Script/Engine.PrimitiveComponent)
    (if (!= _array_element self)
      (Game|Damage|ApplyDamage _array_element (Variables|Default|GetDamage%20Amount) 0 0)
      (Development|PrintString "Hello"))))