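; Game mode Blueprint that respawns the player's PP_Player character after it is destroyed.
; BeginPlay binds to the character's OnDestroyed event, which waits briefly, spawns a new PP_Player and has the first player controller possess it.
; It then calls Respawn, which re-enters the BeginPlay binding so the cycle repeats for each new pawn.
; An alternative respawn chain with a sound is unconnected, and Respawn2 is empty.
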(event Custom|Respawn
  (params (SpawnTransform :type Transform))
  (Utilities|Casting|CastToPP_Player (Game|GetPlayerCharacter 0))
  (Game|BindEventtoOnDestroyed (delegate Custom|OnDestroyed_)))

(event Custom|OnDestroyed_
  (params (DestroyedActor :type Actor%20Object%20Reference))
  (Utilities|FlowControl|Delay 2.0)
  (bind _returnvalue (Game|SpawnActorfromClass "/Game/Blueprints/PP_Player.PP_Player_C" (Variables|Default|GetSpawn%20Transform) "Undefined" "MultiplyWithRoot" 0 0))
  (Pawn|Possess (Game|GetPlayerController 0) _returnvalue)
  (CallFunction|Respawn))

(event Custom|Respawn2)

(event EventBeginPlay
  (Utilities|Casting|CastToPP_Player (Game|GetPlayerCharacter 0))
  (Game|BindEventtoOnDestroyed (delegate Custom|OnDestroyed_)))

(fn ConstructionScript)