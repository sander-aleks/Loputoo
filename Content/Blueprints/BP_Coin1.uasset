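; BP_Coin1 is a coin pickup that adds one to the Coins count of PP_Player.
; A box overlap by that player increments the count, plays a 2D sound and destroys the coin.
; On BeginPlay a self-restarting timeline sets the coin's world rotation each update, keeping its initial roll and pitch.
; Yaw is a constant zero with no timeline track feeding it, so the file shows no actual spin.
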(event OnComponentBeginOverlap(Box)
  (params (OverlappedComponent :type Primitive%20Component%20Object%20Reference) (OtherActor :type Actor%20Object%20Reference) (OtherComp :type Primitive%20Component%20Object%20Reference) (OtherBodyIndex :type Integer) (bFromSweep :type Boolean) (SweepResult :type Hit%20Result%20Structure%20%28by%20ref%29))
  (bind _aspp_player (Utilities|Casting|CastToPP_Player OtherActor))
  (Variables|/Game/Blueprints/PP_Player.PP_Player_C|SetCoins _aspp_player (+ (Variables|/Game/Blueprints/PP_Player.PP_Player_C|GetCoins _aspp_player) 1))
  (Audio|PlaySound2D "/Game/Sound/sound1.sound1" 0.2 1.0 0.0 0 0)
  (Actor|DestroyActor))

(event EventBeginPlay
  (Variables|Default|SetNewVar (Transformation|GetWorldRotation (Variables|Default|GetCoin)))
  (Timeline|Timeline Play
    (:Update
      (Transformation|SetWorldRotation (Variables|Default|GetCoin) (Math|Rotator|MakeRotator (.roll (Variables|Default|GetNewVar)) (.pitch (Variables|Default|GetNewVar)) 0.0) false false))
    (:Finished
      (Timeline|Timeline PlayFromStart))))

(fn ConstructionScript)